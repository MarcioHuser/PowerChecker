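; Blueprint function library of logging, text and value helpers for PowerChecker.
; The info, warning and error loggers share BuildMessage, which prefixes messages with time and the actor's path name.
; All three levels require Enabled, plus either ForceLog or the info-log check, even for warnings and errors.
; Other helpers pick a valid class, convert booleans or text, and format per-minute values, showing "--" when they round to zero.
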(fn `booleanToText`
  (params (value :type Boolean) (true :type Text :default "NSLOCTEXT(\"[25DE7F3C477A551A0269A48868FEE2C6]\", \"D0AE2C3C46EA2586DEDF53865D77F274\", \"True\")") (false :type Text :default "NSLOCTEXT(\"[25DE7F3C477A551A0269A48868FEE2C6]\", \"8565C42C4752F60440A15CA293732D35\", \"False\")"))
  (returns (text :type Text))
  (return (select `bool` value :`false` false :`true` true)))

(fn `buildMessage`
  (params (actor :type "Actor Object Reference") (inMessage :type Text) (inEnabled :type Boolean :default true) (forceLog :type Boolean))
  (returns (outMessage :type String) (outEnabled :type Boolean))
  (if (and inEnabled (or (and (not forceLog) (`PowerCheckerLogic.IsLogInfoEnabled`)) forceLog))
    (return (`KismetTextLibrary.Conv_TextToString` (`|FormatText` "{time} {path}: {message}" (`self.getNowTime` null) (`self.getPathNameText` actor) inMessage)) true)
    (else
      (return "" false))))

(fn `formatPerMinute`
  (params (Value :type "Float (double-precision)"))
  (returns (ReturnValue :type Text))
  (return (select `bool` (!= (`FGBlueprintFunctionLibrary.RoundFloatWithPrecision` Value 4) 0.0) :`false` "--" :`true` (`KismetTextLibrary.Conv_DoubleToText` Value "HalfToEven" false true 1 324 0 4))))

(fn `getNowTime`
  (returns (ReturnValue :type Text))
  (return (`KismetTextLibrary.AsTime_DateTime` (`KismetMathLibrary.Now`))))

(fn `getPathNameText`
  (params (Object :type "Object Object Reference"))
  (returns (ReturnValue :type Text))
  (return (`KismetTextLibrary.Conv_StringToText` (`KismetSystemLibrary.GetPathName` Object))))

(fn `getValidItem`
  (params (value1 :type "FGItemDescriptor Class Reference") (value2 :type "FGItemDescriptor Class Reference"))
  (returns (return :type "FGItemDescriptor Class Reference"))
  (return (select `bool` (`KismetSystemLibrary.IsValidClass` value1) :`false` value2 :`true` value1)))

(fn `logErrorPrefixed`
  (params (actor :type "Actor Object Reference") (message :type Text) (enabled :type Boolean :default true) (forceLog :type Boolean))
  (bind (_outmessage _outenabled) (`self.buildMessage` actor message enabled forceLog))
  (if _outenabled
    (`SMLBlueprintLibrary.LogError` _outmessage)))

(fn `logInfoPrefixed`
  (params (actor :type "Actor Object Reference") (message :type Text) (enabled :type Boolean :default true) (forceLog :type Boolean))
  (bind (_outmessage _outenabled) (`self.buildMessage` actor message enabled forceLog))
  (if _outenabled
    (`SMLBlueprintLibrary.LogInfo` _outmessage)))

(fn `logWarningPrefixed`
  (params (actor :type "Actor Object Reference") (message :type Text) (enabled :type Boolean :default true) (forceLog :type Boolean))
  (bind (_outmessage _outenabled) (`self.buildMessage` actor message enabled forceLog))
  (if _outenabled
    (`SMLBlueprintLibrary.LogWarning` _outmessage)))

(fn `textToFloat`
  (params (text :type Text) (maximumFractionalDigits :type Integer :default 8))
  (returns (float :type "Float (double-precision)"))
  (return (`FGBlueprintFunctionLibrary.RoundFloatWithPrecision` (`KismetStringLibrary.Conv_StringToDouble` (`KismetTextLibrary.Conv_TextToString` text)) maximumFractionalDigits)))